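; BP_APICALL is a test Blueprint that queries the NFTPort API for the NFTs of a hard-coded wallet on the Rinkeby chain.
; Pressing X builds a VaRest GET request with an inline authorization key and sends it.
; On completion it loops over the "nfts" array and prints each contract address to screen.
; On failure it prints only a placeholder "Hello", and BeginPlay and Tick are empty.
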(event `Key|X`
  (params (Key :type "Key Structure"))
  (:`Pressed`
    (bind _returnvalue (`VaRestSubsystem.ConstructVaRestRequestExt` (subsystem `VaRestSubsystem`) "GET" "x_www_form_urlencoded_url"))
    (`VaRestRequestJSON.SetHeader` _returnvalue "Authorization" "a3f41a11-53f9-47ff-aeef-c2bbe67b2562")
    (`VaRestRequestJSON.SetHeader` _returnvalue "Content-Type" "application/json")
    (add `VaRestRequestJSON.OnRequestComplete` _returnvalue (delegate `CustomEvent_0`))
    (add `VaRestRequestJSON.OnRequestFail` _returnvalue (delegate `CustomEvent_1`))
    (`VaRestRequestJSON.ProcessURL` _returnvalue "https://api.nftport.xyz/v0/accounts/0xc3B67AA8358eEA8C4C3df888199999E2193F1993?chain=rinkeby&include=default")))

(event `self.ReceiveBeginPlay`)

(event `CustomEvent_1`
  (params (Request :type "VaRestRequestJSON Object Reference"))
  (`KismetSystemLibrary.PrintString` "Hello"))

(event `CustomEvent_0`
  (params (Request :type "VaRestRequestJSON Object Reference"))
  (for _array_element (`VaRestJsonObject.GetArrayField` (`VaRestRequestJSON.GetResponseObject` Request) "nfts")
    (bind _returnvalue (`VaRestJsonValue.AsObject` _array_element))
    (`KismetSystemLibrary.PrintString` (`VaRestJsonObject.GetStringField` _returnvalue "contract_address") true true (struct :`G` 0.66 :`B` 1.0 :`A` 1.0) 10.0)))