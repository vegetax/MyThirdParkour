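; BP_Cargo is a physics-simulated cargo actor for the crane package, meant to be carried by and released from a hook.
; Its construction script assigns a configurable static mesh and collision object type to the mesh component and turns on physics simulation.
; An AddImpulse function pushes the mesh when the cargo detaches from the hook, and the event graph holds no active logic.
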(fn `AddImpulse`
  (params (Impulse :type "Vector Structure") (bVelChange :type Boolean))
  ;[1 1 1] Add impule when cargo detach from hook
  (`PrimitiveComponent.AddImpulse` (`self.SM_Mesh`) Impulse "None" bVelChange))

(fn `UserConstructionScript`
  ;[1 1 1] Setup Mesh Settings
  (`StaticMeshComponent.SetStaticMesh` (`self.SM_Mesh`) (`self.MeshRef`))
  (`PrimitiveComponent.SetCollisionObjectType` (`self.SM_Mesh`) (`self.ObjectType`))
  (`PrimitiveComponent.SetSimulatePhysics` (`self.SM_Mesh`) true))