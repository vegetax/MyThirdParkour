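; Crane magnet actor that grabs and releases physics-simulated cargo.
; HookAction toggles: it releases held cargo, or box-traces down from Trace_Socket, sized by the mesh bounds, for a configured object type.
; A simulating hit is swept to the actor's location and joined to the magnet mesh by a physics constraint.
; UnhookAction breaks the constraint and clears Attached; the trace leaves debug drawing on.
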(event `/Game/Packages/Crane/Blueprints/Interface/BPI_HookAction.UnhookAction`
  ;[1 1 1] Dump cargo from hook
  (set `self.bAttached` false :!label _label)
  (`PhysicsConstraintComponent.BreakConstraint` (`self.PhysicsConstraint`)))

(event `/Game/Packages/Crane/Blueprints/Interface/BPI_HookAction.HookAction`
  (bind _staticmesh (`self.StaticMesh`))
  (bind _returnvalue (`SceneComponent.GetSocketLocation` _staticmesh "Trace_Socket"))
  ;[1 1 1] Check attached cargo
  (if (`self.bAttached`)
    (goto _label)
    (else
      ;[1 1 1] If the object is suitable for this type and physical modeling is enabled for it, then grab it.
      (bind (_outhit _returnvalue_2) (`KismetSystemLibrary.BoxTraceSingleForObjects` :`Start` _returnvalue :`End` (+ _returnvalue (* (* (`SceneComponent.GetUpVector` _staticmesh) -1.0) (`self.TraceLength`))) :`HalfSize` (`.BoxExtent` (`KismetSystemLibrary.GetComponentBounds` _staticmesh)) :`ObjectTypes` (`self.ObjectsTypeTrace`) :`DrawDebugType` "ForDuration"))
      (if _returnvalue_2
        (bind (_bblockinghit _binitialoverlap _time _distance _location _impactpoint _normal _impactnormal _physmat _hitactor _hitcomponent) (`GameplayStatics.BreakHitResult` _outhit))
        (if (`SceneComponent.IsSimulatingPhysics` _hitcomponent "None")
          (`SceneComponent.K2_SetWorldLocation` _hitcomponent (`self.K2_GetActorLocation`) true true)
          (`PhysicsConstraintComponent.SetConstrainedComponents` (`self.PhysicsConstraint`) (`self.StaticMesh`) "None" _hitcomponent "None")
          (set `self.bAttached` true))))))

(fn `UserConstructionScript`
  (`parent.UserConstructionScript`))