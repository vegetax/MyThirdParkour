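; BP_MedievalHook is a crane hook actor that picks up and releases BP_Cargo actors.
; With SnapToCargo on, HookAction sphere-traces below the hook socket, attaches the cargo found there and aligns it with a yaw offset.
; UnhookAction detaches snapped cargo, nudges the hook upward and passes its velocity to the cargo as an impulse.
; With no snapped cargo, unhooking only raises the hook, freeing physically hooked loads.
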(event `/Game/Packages/Crane/Blueprints/Interface/BPI_HookAction.HookAction`
  (bind _staticmesh (`self.StaticMesh`))
  (bind (_returnvalue_roll _returnvalue_pitch _returnvalue_yaw) (`KismetMathLibrary.BreakRotator` (`SceneComponent.GetSocketRotation` (`self.StaticMesh`) "Hook_Socket")))
  (bind _returnvalue (`SceneComponent.GetSocketLocation` _staticmesh "Hook_Socket"))
  (`/Engine/EditorBlueprintResources/StandardMacros.IsValid` (`self.CargoActorRef`) ; if there is a cargo we do nothing
    (:`Is Not Valid`
      (if (`self.bSnapToCargo`)
        ;[1 1 1] Check type object, BP_Cargo and if everything is correctly attach the cargo to the hook
        (bind (_outhit _returnvalue_2) (`KismetSystemLibrary.SphereTraceSingleForObjects` :`Start` _returnvalue :`End` (+ _returnvalue (* (* (`SceneComponent.GetUpVector` _staticmesh) -1.0) (`self.TraceLength`))) :`Radius` (`self.HookRadiusAction`) :`ObjectTypes` (`self.ObjectsTypeTrace`) :`DrawDebugType` "ForDuration"))
        (if _returnvalue_2
          (bind _asbp_cargo (cast `/Game/Packages/Crane/Blueprints/BP_Cargo` (`.HitActor` (`GameplayStatics.BreakHitResult` _outhit))))
          (bind _output_get (set `self.CargoActorRef` _asbp_cargo))
          (`self.K2_AttachToActor` _output_get self "Hook_Socket" "SnapToTarget" "KeepRelative" "KeepRelative" true)
          (`self.K2_SetActorRotation` (struct))
          (`self.K2_SetActorRotation` (`self.CargoActorRef`) (`KismetMathLibrary.MakeRotator` _returnvalue_roll _returnvalue_pitch (+ _returnvalue_yaw (`self.YawOffsetCargo`))) false))))))

(event `/Game/Packages/Crane/Blueprints/Interface/BPI_HookAction.UnhookAction`
  ;[1 1 1] Unhook actor (detach)
  (if (`self.bSnapToCargo`)
    ;;[1 1 1] By snap
    (`/Engine/EditorBlueprintResources/StandardMacros.IsValid` (`self.CargoActorRef`)
      (:`Is Valid`
        (`self.DetachActor` 50.0)
        (`/Game/Packages/Crane/Blueprints/BP_Cargo.AddImpulse` (`self.CargoActorRef`) (`self.GetVelocity`) true)
        (set `self.CargoActorRef` null))
      (:`Is Not Valid`
        ;;[1 1 1] By physics
        (`self.RemoveFromHook` 50.0 :!label _label)))
    (else
      (goto _label))))

(fn `DetachActor`
  (params (Z :type "Float (double-precision)" :default 50.0))
  ;[1 1 1] Detach cargo from hook
  (`self.K2_DetachFromActor` (`self.CargoActorRef`) "KeepWorld" "KeepWorld" "KeepWorld")
  (`self.RemoveFromHook` Z))

(fn `RemoveFromHook`
  (params (Z :type "Float (double-precision)" :default 50.0))
  ;[1 1 1] Slightly raise the hook up
  (`self.K2_SetActorLocation` (+ (`self.K2_GetActorLocation`) (`KismetMathLibrary.MakeVector` 0.0 0.0 Z)) false true))

(fn `UserConstructionScript`
  (`parent.UserConstructionScript`))