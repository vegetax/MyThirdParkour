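; BP_Crane is a player-controllable crane with a rotating top, pitching arm, orbit camera and variable-length cable.
; StartControl and EndControl switch view, input and UI between pawn and crane.
; The hook is a swappable BP_BaseHook child actor (hook, magnet, platform, medieval hook, double ladle) receiving action inputs.
; A physics constraint hangs it from the arm, its Z limit following the interpolated cable length, while an optional downward trace drives a beam and decal.
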(event `self.ReceiveBeginPlay`
  ;[1 1 1] Initialize
  ;;[1 1 1] Check valid hook
  (`/Engine/EditorBlueprintResources/StandardMacros.IsValid` (`self.HookRef`)
    (:`Is Valid`
      ;;[1 1 1] Set location start hook
      (`self.K2_SetActorLocation` (`self.HookRef`) (- (`SceneComponent.GetSocketLocation` (`self.SM_CraneArrow`) "Cable_Socket") (0.0 0.0 150.0)) false false)
      ;;[1 1 1] Set constrained to hook
      (`PhysicsConstraintComponent.SetConstrainedComponents` (`self.CraneArrowConstrain`) (`self.SM_CraneArrow`) "None" (`/Game/Packages/Crane/Blueprints/BP_BaseHook.StaticMesh` (cast `/Game/Packages/Crane/Blueprints/BP_BaseHook` (`self.HookRef`) :!pure true)) "Hook_Socket")
      ;;[1 1 1] Attach cable end to hook
      (`CableComponent.SetAttachEndTo` (`self.Cable`) (`self.HookRef`) "StaticMesh" "None")
      ;;[1 1 1] Set hook owner
      (`self.SetOwner` (`self.HookRef`) self))))

(event `InputAxis|LookUpCameraCrane`
  (params (AxisValue :type "Float (single-precision)"))
  ;[1 1 1] Camera
  (`SceneComponent.K2_AddRelativeRotation` (`self.SpringArm`) (`KismetMathLibrary.MakeRotator` 0.0 (* AxisValue (`self.LookUpCameraSpeed`))) false false))

(event `self.ReceiveTick`
  (params (DeltaSeconds :type "Float (single-precision)"))
  (bind _hookref (`self.HookRef`))
  (bind _returnvalue (`self.K2_GetActorLocation` _hookref))
  (bind _returnvalue_2 (`KismetMathLibrary.FClamp` (`KismetMathLibrary.FInterpTo` (`CableComponent.CableLength` (`self.Cable`)) (`self.CableLength`) (`GameplayStatics.GetWorldDeltaSeconds`) (`self.CableChangeSmoothLengthSpeed`)) (`self.CableLengthMin`) (`self.CableLengthMax`)))
  ;[1 1 1] Smooth Change cable length
  (`|ExecutionSequence`
    (:`then_0`
      ;[1 1 1] Update hook tracer
      (if (`self.bShowTracerIfPlayerControl`)
        (`/Engine/EditorBlueprintResources/StandardMacros.IsValid` _hookref
          (:`Is Valid`
            (bind (_outhit _returnvalue_3) (`KismetSystemLibrary.LineTraceSingleForObjects` _returnvalue (- _returnvalue (0.0 0.0 10000.0)) (`|MakeArray` "ObjectTypeQuery1" :!type "EObjectTypeQuery Enum")))
            (if _returnvalue_3
              (bind (_bblockinghit _binitialoverlap _time _distance _location) (`GameplayStatics.BreakHitResult` _outhit))
              (`SceneComponent.K2_SetWorldLocation` (`self.Decal`) _location false false)
              (`ParticleSystemComponent.SetBeamTargetPoint` (`self.P_HookTracer`) 0 _location 0)
              (`SceneComponent.K2_SetWorldLocation` (`self.P_HookTracer`) (`self.K2_GetActorLocation` (`self.HookRef`)) false false))))))
    (:`then_1`
      (set `CableComponent.CableLength` _returnvalue_2 (`self.Cable`))
      (`PhysicsConstraintComponent.SetLinearZLimit` (`self.CraneArrowConstrain`) "LCM_Limited" (+ _returnvalue_2 20.0)))))

(event `InputAxis|TurnCameraCrane`
  (params (AxisValue :type "Float (single-precision)"))
  ;[1 1 1] Camera
  (`SceneComponent.K2_AddRelativeRotation` (`self.SpringArm`) (`KismetMathLibrary.MakeRotator` 0.0 0.0 (* AxisValue (`self.TurnCameraSpeed`))) false false))

(event `InputAction|NextHook`
  (params (Key :type "Key Structure"))
  (bind _returnvalue (`KismetMathLibrary.Conv_ByteToInt` (`self.TypeHook`)))
  ;[1 1 1] Switch to next hook. Hook -> Magnet -> Platform -> MedievalHook -> Hook ...
  (:`Pressed`
    (if (== (- (enumcount `/Game/Packages/Crane/Blueprints/Enumerations/E_TypeHooks`) 1) _returnvalue)
      (set `self.TypeHook` "NewEnumerator0")
      (else
        (set `self.TypeHook` (cast `/Game/Packages/Crane/Blueprints/Enumerations/E_TypeHooks` (`KismetMathLibrary.Conv_IntToByte` (+ _returnvalue 1))))))
    (switch `/Game/Packages/Crane/Blueprints/Enumerations/E_TypeHooks` (`self.TypeHook`)
      (:`NewEnumerator0`
        (set `self.HookClass` "/Game/Packages/Crane/Blueprints/BP_Hook.BP_Hook_C"))
      (:`NewEnumerator1`
        (set `self.HookClass` "/Game/Packages/Crane/Blueprints/BP_Magnet.BP_Magnet_C"))
      (:`NewEnumerator2`
        (set `self.HookClass` "/Game/Packages/Crane/Blueprints/BP_Platform.BP_Platform_C"))
      (:`NewEnumerator3`
        (set `self.HookClass` "/Game/Packages/Crane/Blueprints/BP_MedievalHook.BP_MedievalHook_C"))
      (:`NewEnumerator4`
        (set `self.HookClass` "/Game/Packages/Crane/Blueprints/BP_DoubleLadle.BP_DoubleLadle_C")))
    (`self.UpdateHook`)))

(event `InputAxis|TurnCrane`
  (params (AxisValue :type "Float (single-precision)"))
  ;[1 1 1] Crane mechnic parts
  (`SceneComponent.K2_AddLocalRotation` (`self.SM_CraneTop`) (`KismetMathLibrary.MakeRotator` 0.0 0.0 (* AxisValue (`self.TurnCraneSpeed`) (`GameplayStatics.GetWorldDeltaSeconds`))) false false))

(event `InputAxis|PitchCraneArrow`
  (params (AxisValue :type "Float (single-precision)"))
  (bind _sm_cranearrow (`self.SM_CraneArrow`))
  (bind (_relativerotation_roll _relativerotation_pitch) (`KismetMathLibrary.BreakRotator` (`SceneComponent.RelativeRotation` _sm_cranearrow)))
  ;[1 1 1] Crane mechnic parts
  (`SceneComponent.K2_SetRelativeRotation` _sm_cranearrow (`KismetMathLibrary.MakeRotator` 0.0 (`KismetMathLibrary.FClamp` (+ _relativerotation_pitch (* AxisValue (`self.PitchCraneArrowSpeed`) (`GameplayStatics.GetWorldDeltaSeconds`))) (`self.MinCranePitchArrow`) (`self.MaxCranePitchArrow`))) false false))

(event `InputAxisKey|MouseWheelAxis`
  (params (AxisValue :type "Float (single-precision)"))
  ;[1 1 1] Change cable length by mouse wheel
  (`self.CalculateCableLenght` AxisValue (`self.CableLengthMouseSpeed`)))

(event `InputAction|CraneHookAction`
  (params (Key :type "Key Structure"))
  ;[1 1 1] Hook actor call Action
  (:`Pressed`
    (`/Engine/EditorBlueprintResources/StandardMacros.IsValid` (`self.HookRef`)
      (:`Is Valid`
        (switch `/Game/Packages/Crane/Blueprints/Enumerations/E_TypeHooks` (`self.TypeHook`)
          (:`NewEnumerator0`
            (bind _asbp_base_hook (cast `/Game/Packages/Crane/Blueprints/BP_BaseHook` (`self.HookRef`) :!label _label))
            (`/Game/Packages/Crane/Blueprints/Interface/BPI_HookAction.HookAction` _asbp_base_hook))
          (:`NewEnumerator1`
            (goto _label))
          (:`NewEnumerator2`
            (goto _label))
          (:`NewEnumerator3`
            (goto _label))
          (:`NewEnumerator4`
            (bind _asbp_base_hook_2 (cast `/Game/Packages/Crane/Blueprints/BP_BaseHook` (`self.HookRef`)))
            (`/Game/Packages/Crane/Blueprints/BP_BaseHook.LadleClose` _asbp_base_hook_2 true))))))
  (:`Released`
    (`/Engine/EditorBlueprintResources/StandardMacros.IsValid` (`self.HookRef`)
      (:`Is Valid`
        (switch `/Game/Packages/Crane/Blueprints/Enumerations/E_TypeHooks` (`self.TypeHook`)
          (:`NewEnumerator4`
            (bind _asbp_base_hook_3 (cast `/Game/Packages/Crane/Blueprints/BP_BaseHook` (`self.HookRef`)))
            (`/Game/Packages/Crane/Blueprints/BP_BaseHook.LadleClose` _asbp_base_hook_3 false)))))))

(event `InputAxis|CableLenghtGamepad`
  (params (AxisValue :type "Float (single-precision)"))
  ;[1 1 1] Change cable length by gamepad
  (`self.CalculateCableLenght` AxisValue (`self.CableLengthGamepadSpeed`)))

(event `InputAction|EndControlCrane`
  (params (Key :type "Key Structure"))
  ;[1 1 1] End control crane
  (:`Pressed`
    (`self.EndControl`)))

(event `InputAction|CraneUnhookAction`
  (params (Key :type "Key Structure"))
  ;[1 1 1] Unhook actor call Action
  (:`Pressed`
    (`/Engine/EditorBlueprintResources/StandardMacros.IsValid` (`self.HookRef`)
      (:`Is Valid`
        (switch `/Game/Packages/Crane/Blueprints/Enumerations/E_TypeHooks` (`self.TypeHook`)
          (:`NewEnumerator0`
            (bind _asbp_base_hook (cast `/Game/Packages/Crane/Blueprints/BP_BaseHook` (`self.HookRef`) :!label _label_2))
            (`/Game/Packages/Crane/Blueprints/BP_BaseHook.UnhookAction` _asbp_base_hook))
          (:`NewEnumerator1`
            (goto _label_2))
          (:`NewEnumerator2`
            (goto _label_2))
          (:`NewEnumerator3`
            (goto _label_2))
          (:`NewEnumerator4`
            (bind _asbp_base_hook_2 (cast `/Game/Packages/Crane/Blueprints/BP_BaseHook` (`self.HookRef`)))
            (`/Game/Packages/Crane/Blueprints/BP_BaseHook.LadleOpen` _asbp_base_hook_2 true))))))
  (:`Released`
    (`/Engine/EditorBlueprintResources/StandardMacros.IsValid` (`self.HookRef`)
      (:`Is Valid`
        (switch `/Game/Packages/Crane/Blueprints/Enumerations/E_TypeHooks` (`self.TypeHook`)
          (:`NewEnumerator4`
            (bind _asbp_base_hook_3 (cast `/Game/Packages/Crane/Blueprints/BP_BaseHook` (`self.HookRef`)))
            (`/Game/Packages/Crane/Blueprints/BP_BaseHook.LadleOpen` _asbp_base_hook_3 false)))))))

(fn `DetachHookRef`
  ;[1 1 1] Detach hook. Look "BP_Plathorm" event "UnhookAction"
  (`PhysicsConstraintComponent.BreakConstraint` (`self.CraneArrowConstrain`))
  (`CableComponent.SetAttachEndTo` (`self.Cable`) null "None" "None")
  (set `CableComponent.bAttachEnd` false (`self.Cable`)))

(fn `EndControl`
  (bind _returnvalue (`GameplayStatics.GetPlayerController` 0))
  (bind _returnvalue_2 (`GameplayStatics.GetPlayerPawn` 0))
  ;[1 1 1] End control crane
  (`PlayerController.SetViewTargetWithBlend` _returnvalue _returnvalue_2 1.0 "VTBlend_Cubic" 0.0 false) ; Move camera to Pawn 0
  (`self.EnableInput` _returnvalue_2 _returnvalue) ; Enable Pawn 0 input
  (`self.DisableInput` _returnvalue) ; Disable crane input
  ;[1 1 1] Remove widget input
  (`Widget.RemoveFromParent` (`self.CraneWidgetInputRef`))
  ;[1 1 1] Show again player widget
  (bind _asbp_third_person_character (cast `/Game/Packages/Crane/Demo/ThirdPerson/ThirdPersonBP/Blueprints/BP_ThirdPersonCharacter` (`GameplayStatics.GetPlayerPawn` 0)))
  (`Widget.SetVisibility` (`/Game/Packages/Crane/Demo/ThirdPerson/ThirdPersonBP/Blueprints/BP_ThirdPersonCharacter.PlayerWidgetInputRef` _asbp_third_person_character) "Visible")
  ;[1 1 1] Hide hook tracer
  (if (`self.bUseHookTracer`)
    (set `self.bShowTracerIfPlayerControl` false)
    (`SceneComponent.SetVisibility` (`self.P_HookTracer`) false false)
    (`SceneComponent.SetVisibility` (`self.Decal`) false false)))

(fn `StartControl`
  (params (Target :type "Actor Object Reference"))
  (bind _returnvalue (`GameplayStatics.GetPlayerController` 0))
  ;[1 1 1] Start control crane
  (`PlayerController.SetViewTargetWithBlend` _returnvalue self 1.0 "VTBlend_Cubic" 0.0 false) ; Move camera to crane
  (`self.EnableInput` _returnvalue) ; Enable crane input
  (`self.DisableInput` Target _returnvalue) ; diable input pawn
  ;[1 1 1] Create widget with input
  (bind _returnvalue_2 (`|CreateWidget` "/Game/Packages/Crane/Blueprints/UMG/WBP_CraneInput.WBP_CraneInput_C"))
  (bind _output_get (set `self.CraneWidgetInputRef` _returnvalue_2))
  (`UserWidget.AddToViewport` _output_get 0)
  ;[1 1 1] Show hook tracer
  (if (`self.bUseHookTracer`)
    (set `self.bShowTracerIfPlayerControl` true)
    (`SceneComponent.SetVisibility` (`self.P_HookTracer`) true false)
    (`SceneComponent.SetVisibility` (`self.Decal`) true false)))

(fn `UpdateHook`
  (bind _hookchildactor (`self.HookChildActor`))
  (`ChildActorComponent.SetChildActorClass` _hookchildactor (`self.HookClass`))
  (bind _output_get (set `self.HookRef` (`ChildActorComponent.ChildActor` _hookchildactor)))
  (bind _asbp_base_hook (cast `/Game/Packages/Crane/Blueprints/BP_BaseHook` _output_get))
  (`PhysicsConstraintComponent.SetConstrainedComponents` (`self.CraneArrowConstrain`) (`self.SM_CraneArrow`) "None" (`/Game/Packages/Crane/Blueprints/BP_BaseHook.StaticMesh` _asbp_base_hook) "Hook_Socket")
  (`CableComponent.SetAttachEndTo` (`self.Cable`) (`self.HookRef`) "StaticMesh" "None"))

(fn `UserConstructionScript`
  (`|ExecutionSequence`
    (:`then_1`
      ;[1 1 1] Cable length setting
      (set `self.CableLength` (`KismetMathLibrary.FClamp` (`self.CableLength`) (`self.CableLengthMin`) (`self.CableLengthMax`)))
      (`PhysicsConstraintComponent.SetLinearZLimit` (`self.CraneArrowConstrain`) "LCM_Limited" (`self.CableLength`))
      (set `CableComponent.CableLength` (- (`self.CableLength`) 10.0) (`self.Cable`)))
    (:`then_2`
      ;[1 1 1] Rotate crane arrow
      (`SceneComponent.K2_SetRelativeRotation` (`self.SM_CraneArrow`) (`KismetMathLibrary.MakeRotator` 0.0 (`self.RotateCraneArrow`)) false false))
    (:`then_3`
      ;[1 1 1] Hook setup if HookRef is valid
      (switch `/Game/Packages/Crane/Blueprints/Enumerations/E_TypeHooks` (`self.TypeHook`)
        (:`NewEnumerator0`
          (set `self.HookClass` "/Game/Packages/Crane/Blueprints/BP_Hook.BP_Hook_C"))
        (:`NewEnumerator1`
          (set `self.HookClass` "/Game/Packages/Crane/Blueprints/BP_Magnet.BP_Magnet_C"))
        (:`NewEnumerator2`
          (set `self.HookClass` "/Game/Packages/Crane/Blueprints/BP_Platform.BP_Platform_C"))
        (:`NewEnumerator3`
          (set `self.HookClass` "/Game/Packages/Crane/Blueprints/BP_MedievalHook.BP_MedievalHook_C"))
        (:`NewEnumerator4`
          (set `self.HookClass` "/Game/Packages/Crane/Blueprints/BP_DoubleLadle.BP_DoubleLadle_C")))
      (`SceneComponent.K2_SetWorldTransform` (`self.HookChildActor`) (`KismetMathLibrary.MakeTransform` (- (`SceneComponent.GetSocketLocation` (`self.SM_CraneArrow`) "Cable_Socket") (0.0 0.0 50.0))) false false)
      (`self.UpdateHook`))))