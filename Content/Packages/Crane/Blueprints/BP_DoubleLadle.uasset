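; BP_DoubleLadle is a two-part crane ladle whose left and right meshes swing open and closed.
; LadleClose and LadleOpen set the animation direction and toggle Tick with their Enable flag, unless the ladle is already at that limit.
; Tick advances a speed-scaled alpha, lerps both meshes' relative roll between open and closed angles, then disables itself at either end.
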(event `self.ReceiveTick`
  (params (DeltaSeconds :type "Float (single-precision)"))
  (switch `ETimelineDirection` (`self.DirectionAnimation`)
    (:`Forward`
      (`SceneComponent.K2_SetRelativeRotation` (`self.SM_LeftLadle`) (`KismetMathLibrary.MakeRotator` (`KismetMathLibrary.Lerp` 100.0 0.0 (`self.StateLadleAnimation`))) false false)
      (`SceneComponent.K2_SetRelativeRotation` (`self.SM_RightLadle`) (`KismetMathLibrary.MakeRotator` (`KismetMathLibrary.Lerp` 100.0 0.0 (`self.StateLadleAnimation`))) false false)
      (bind _output_get (set `self.StateLadleAnimation` (+ (`self.StateLadleAnimation`) (* (`GameplayStatics.GetWorldDeltaSeconds`) (`self.SpeedAnimation`)))))
      (if (>= _output_get 1.0)
        (`self.SetActorTickEnabled` false)))
    (:`Backward`
      (`SceneComponent.K2_SetRelativeRotation` (`self.SM_LeftLadle`) (`KismetMathLibrary.MakeRotator` (`KismetMathLibrary.Lerp` 100.0 0.0 (`self.StateLadleAnimation`))) false false)
      (`SceneComponent.K2_SetRelativeRotation` (`self.SM_RightLadle`) (`KismetMathLibrary.MakeRotator` (`KismetMathLibrary.Lerp` 100.0 0.0 (`self.StateLadleAnimation`))) false false)
      (bind _output_get_2 (set `self.StateLadleAnimation` (- (`self.StateLadleAnimation`) (* (`GameplayStatics.GetWorldDeltaSeconds`) (`self.SpeedAnimation`)))))
      (if (<= _output_get_2 0.0)
        (`self.SetActorTickEnabled` false)))))

(event `/Game/Packages/Crane/Blueprints/Interface/BPI_HookAction.LadleClose`
  (params (Enable :type Boolean))
  (if (< (`self.StateLadleAnimation`) 1.0)
    (set `self.DirectionAnimation` "Forward")
    (`self.SetActorTickEnabled` Enable)))

(event `/Game/Packages/Crane/Blueprints/Interface/BPI_HookAction.LadleOpen`
  (params (Enable :type Boolean))
  (if (> (`self.StateLadleAnimation`) 0.0)
    (set `self.DirectionAnimation` "Backward")
    (`self.SetActorTickEnabled` Enable)))

(fn `UserConstructionScript`
  (`parent.UserConstructionScript`))