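; Power line actor that builds a row of electrical poles with sagging, swaying cables from a list of transforms.
; The construction script adds an instanced pole per location and strings six cable components back to the previous pole.
; Hardcoded height and sideways offsets stand in for sockets, which instanced meshes lack, and cable lengths derive from span distance with random variation.
; Tick applies a sine-driven sideways force to every cable.
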(event `self.ReceiveTick`
  (params (DeltaSeconds :type "Float (single-precision)"))
  (for _array_element (`self.Cables`)
    (set `CableComponent.CableForce` (`KismetMathLibrary.MakeVector` 0.0 (* (`KismetMathLibrary.DegSin` (* (`KismetSystemLibrary.GetGameTimeInSeconds`) 90.0)) 700.0)) _array_element)))

(fn `UserConstructionScript`
  (locals (CoilDistance :type "Float (double-precision)" :default 0.0) (CurrentInstance :type Integer))
  (bind _outinstancetransform (`InstancedStaticMeshComponent.GetInstanceTransform` (`self.PoleInstances`) (`local.CurrentInstance`) false))
  (bind _outinstancetransform_2 (`InstancedStaticMeshComponent.GetInstanceTransform` (`self.PoleInstances`) (- (`local.CurrentInstance`) 1) false))
  ;[1 1 1] Go through all of the locations to add a Pole
  (for _array_element (`self.Locations`)
    (bind _returnvalue (`InstancedStaticMeshComponent.AddInstance` (`self.PoleInstances`) _array_element false))
    (set `local.CurrentInstance` _returnvalue) ; Set the current Instance Index
    (if (!= _returnvalue 0)
      (for _index (range 1 7)
        (set `local.CoilDistance` (select `int` _index :`0` 0.0 :`1` 165.0 :`2` 100.0 :`3` 39.0 :`4` -39.0 :`5` -100.0 :`6` -165.0)) ; Unfortunately we can't get sockets on Instanced Meshes, so we're getting offsets for the coils
        (bind _returnvalue_2 (`AddComponent|NODE_AddCableComponent-0` :`RelativeTransform` (`KismetMathLibrary.MakeTransform` (+ (.location _outinstancetransform) (0.0 0.0 870.0) (* (`KismetMathLibrary.GetRightVector` (.rotation _outinstancetransform)) (`local.CoilDistance`))))))
        (set `CableComponent.EndLocation` (+ (.location _outinstancetransform_2) (0.0 0.0 870.0) (* (`KismetMathLibrary.GetRightVector` (.rotation _outinstancetransform_2)) (`local.CoilDistance`))) _returnvalue_2) ; Set the end location using the last pole's location (w/ offsets)
        (set `CableComponent.CableLength` (+ (`KismetMathLibrary.Vector_Distance` (`SceneComponent.RelativeLocation` _returnvalue_2) (`CableComponent.EndLocation` _returnvalue_2)) (`KismetMathLibrary.RandomFloatInRange` -40.0 40.0) -60.0) _returnvalue_2) ; Set the cable length based on the distance from the start and end of the cable
        (`KismetArrayLibrary.Array_Add` (`self.Cables`) _returnvalue_2)))))